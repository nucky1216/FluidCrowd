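; Test actor that drives a grid-based Niagara system and sets its target cell by mouse picking.
; The construction script passes grid resolution, size and target position to Niagara.
; Ctrl+left-click traces the Visibility channel under the cursor, logs the hit and draws a debug point.
; PosToGridIndex converts the hit into actor-local, center-offset X/Y cell indices with Z zeroed, which become Niagara's TargetPos.
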(event EventBeginPlay)

(event Collision|EventActorBeginOverlap
  (params (OtherActor :type Actor%20Object%20Reference)))

(event EventTick
  (params (DeltaSeconds :type Float%20%28single-precision%29)))

(event Input|MouseEvents|CtrlLeftMouseButton
  (params (Key :type Key%20Structure :default "None"))
  (bind _returnvalue (Game|GetPlayerController 0))
  (bind (_posx _posy) (Class|VictoryBPFunctionLibrary|ViewportGetMousePosition _returnvalue))
  (:Pressed
    (bind _outhitresult (Class|VictoryBPFunctionLibrary|GetViewportPositionHitResultbyChannel (Math|Vector2D|MakeVector2D _posx _posy) "ECC_Visibility" true))
    (Class|DimensioBPLibrary|PrintLog (Utilities|String|Append (Utilities|GetDisplayName (.HitActor (Collision|BreakHitResult _outhitresult))) ":" (Utilities|String|ToString(Boolean) (.bBlockingHit (Collision|BreakHitResult _outhitresult))) (Utilities|String|ToString(Vector) (CallFunction|PostoGridIndex (.Location (Collision|BreakHitResult _outhitresult))))))
    (Rendering|Debug|DrawDebugPoint (.Location (Collision|BreakHitResult _outhitresult)) 3e+01 "(R=1.000000,G=0.000000,B=0.000000,A=1.000000)" 5.0)
    (Class|NiagaraComponent|SetNiagaraVariableVec3 (Variables|Default|GetNiagara) "TargetPos" (CallFunction|PostoGridIndex (.Location (Collision|BreakHitResult _outhitresult))))))

(fn ConstructionScript
  (CallFunction|SetNiagara))

(fn SetNiagara
  (bind _niagara (Variables|Default|GetNiagara))
  (bind _classprop (Variables|Default|GetClassprop))
  (bind (_gridres _gridsize _targetpos) (Utilities|Struct|BreakS_GridClassprop _classprop))
  (Niagara|SetNiagaraVariable(Vector3) _niagara "GridRes" _gridres)
  (Niagara|SetNiagaraVariable(Vector3) _niagara "GridSize" _gridsize)
  (Niagara|SetNiagaraVariable(Vector3) _niagara "TargetPos" _targetpos))

(fn PostoGridIndex
  (params (Pos :type Vector))
  (bind _returnvalue (Transformation|GetActorTransform))
  (bind _classprop (Variables|Default|GetClassprop))
  (bind (_gridres _gridsize) (Utilities|Struct|BreakS_GridClassprop _classprop))
  (bind _returnvalue_2 (Math|Transform|InvertTransform _returnvalue))
  (bind _returnvalue_3 (Math|Transform|TransformLocation _returnvalue_2 Pos))
  (bind _returnvalue_4 (/ _gridsize _gridres))
  (bind _returnvalue_5 (/ _gridsize 2.0))
  (bind _returnvalue_6 (+ _returnvalue_3 _returnvalue_5))
  (bind _returnvalue_7 (/ _returnvalue_6 _returnvalue_4))
  (bind (_x _y _z) (Math|Vector|BreakVector _returnvalue_7))
  (LocalVariables|SetReCenter _returnvalue_6)
  (return (Math|Vector|MakeVectorNetQuantize (Math|Conversions|ToFloat(Integer) (Math|Float|Floor _x)) (Math|Conversions|ToFloat(Integer) (Math|Float|Floor _y)) 0.0)))